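; BP_Character is a player character that sets up the main HUD and changes the screen look during ultimate abilities.
; On BeginPlay it adds W_MainHUD to the viewport and caches the post-process settings as the normal look.
; Ultimate and teleport-ultimate events swap in distinct color-grading presets, and StopUltimate restores the cached settings.
; The construction script uses UseFirstPersonView to choose whether the first-person camera or the spring-arm third-person camera auto-activates.
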(event `self.ReceiveBeginPlay`
  (`|ExecutionSequence`
    (:`then_0`
      (bind _returnvalue (`|CreateWidget` "/Game/Blueprints/UI/HUD/W_MainHUD.W_MainHUD_C"))
      (`UserWidget.AddToViewport` _returnvalue 0))
    (:`then_1`
      (set `self.NormalPostProcess` (`PostProcessComponent.Settings` (`self.PostProcess`))))))

(event `self.BP_StartUltimate`
  (set `PostProcessComponent.Settings` (make `PostProcessSettings` :`WhiteTemp` 10000.0 :`FilmSlope` 1.5 :`FilmBlackClip` 0.05) (`self.PostProcess`)))

(event `self.BP_StopUltimate`
  (set `PostProcessComponent.Settings` (`self.NormalPostProcess`) (`self.PostProcess`)))

(event `self.BP_StartTeleportUltimate`
  (set `PostProcessComponent.Settings` (make `PostProcessSettings` :`WhiteTemp` 5000.0 :`FilmSlope` 1.5 :`FilmBlackClip` 0.05 :`FilmWhitePoint` (struct :`R` 0.121041 :`G` 0.920303 :`B` 1.0 :`A` 1.0) :`VignetteIntensity` 0.8) (`self.PostProcess`)))

(fn `UserConstructionScript`
  (`ActorComponent.SetAutoActivate` (`self.FPSCameraComponent`) (`self.bUseFirstPersonView`))
  (`ActorComponent.SetAutoActivate` (`self.TPSCameraComponent`) (not (`self.bUseFirstPersonView`)))
  (`ActorComponent.SetAutoActivate` (`self.SpringArmComponent`) (not (`self.bUseFirstPersonView`))))