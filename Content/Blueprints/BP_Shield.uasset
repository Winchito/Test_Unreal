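; BP_Shield is a shield actor that animates a dissolve effect on its mesh when it spawns and when it is destroyed.
; On BeginPlay, a timeline drives the DissolveAmount parameter of a dynamic material instance on the shield mesh.
; The Destroy event creates an instance again and drives the same parameter with a second timeline.
; Its update chains into a short Delay, so the actor is destroyed shortly after that dissolve starts.
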(event `self.ReceiveBeginPlay`
  (bind _returnvalue (`PrimitiveComponent.CreateDynamicMaterialInstance` (`self.ShieldMeshComponent`) 0 null "None"))
  (bind (_direction _newtrack_0) (`Timeline|Timeline_0`)
    (:`Update`
      (`MaterialInstanceDynamic.SetScalarParameterValue` _returnvalue "DissolveAmount" _newtrack_0))))

(event `self.BP_Destroy`
  (bind _returnvalue (`PrimitiveComponent.CreateDynamicMaterialInstance` (`self.ShieldMeshComponent`) 0 null "None"))
  (bind (_direction _newtrack_0) (`Timeline|Timeline_1`)
    (:`Update`
      (`MaterialInstanceDynamic.SetScalarParameterValue` _returnvalue "DissolveAmount" _newtrack_0)
      (`KismetSystemLibrary.Delay` 0.5)
      (`self.K2_DestroyActor`))))

(fn `UserConstructionScript`)